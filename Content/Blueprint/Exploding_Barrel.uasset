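; Exploding barrel actor that detonates when hit by a Laser or when its health runs out.
; A Laser overlap activates its particle system, then runs a delayed, staged blast with emitters, sound, camera shakes and a spawned Explosion actor before destroying itself.
; Separately, damage lowers Health, which Tick polls to trigger a simpler death with one emitter and a sound played at world origin, without spawning an Explosion.
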(event `self.ReceiveAnyDamage`
  (params (Damage :type "Float (single-precision)") (DamageType :type "DamageType Object Reference") (InstigatedBy :type "Controller Object Reference") (DamageCauser :type "Actor Object Reference"))
  (bind _output_get (set `self.Health` (- (`self.Health`) Damage)))
  (`KismetSystemLibrary.PrintString` (`KismetStringLibrary.Concat_StrStr` "Health:" (`KismetStringLibrary.Conv_DoubleToString` _output_get) "Loc:")))

(event `self.ReceiveTick`
  (params (DeltaSeconds :type "Float (single-precision)"))
  ;[1 1 1] Event Tick
  ;[1 1 1] Check For Actor Death
  (if (<= (`self.Health`) 0.0)
    (`self.EnemyDeath`)))

(event `EnemyDeath`
  (`GameplayStatics.PlaySoundAtLocation` "/Game/sound/S_Explode_Reverb_04.S_Explode_Reverb_04")
  (`GameplayStatics.SpawnEmitterAtLocation` "/Game/VFX_Toolkit_V1/ParticleSystems/356Days/Par_Meteora_Explode_01.Par_Meteora_Explode_01" (`self.K2_GetActorLocation`))
  (`self.K2_DestroyActor`))

(event `DamageHealth`
  (set `self.Health` (- (`self.Health`) (`self.DamageAmount`))))

(event `self.collision.OnComponentBeginOverlap`
  (params (OverlappedComponent :type "PrimitiveComponent Object Reference") (OtherActor :type "Actor Object Reference") (OtherComp :type "PrimitiveComponent Object Reference") (OtherBodyIndex :type Integer) (bFromSweep :type Boolean) (SweepResult :type "HitResult Structure (by ref)"))
  (bind _returnvalue (`SceneComponent.K2_GetComponentLocation` (`self.Barrel`)))
  (cast `/Game/Blueprint/Laser` OtherActor)
  (`ActorComponent.Activate` (`self.ParticleSystem`) false)
  (`KismetSystemLibrary.Delay` 1.0)
  (`GameplayStatics.SpawnEmitterAtLocation` "/Game/VFX_Toolkit_V1/ParticleSystems/356Days/Par_MatraBoom_01.Par_MatraBoom_01" _returnvalue (`KismetMathLibrary.Conv_VectorToRotator` _returnvalue) (2.0 2.0 2.0))
  (`GameplayStatics.SpawnSoundAtLocation` "/Game/sound/SC_MissileExplosion.SC_MissileExplosion" _returnvalue (`KismetMathLibrary.Conv_VectorToRotator` _returnvalue) 10.0 0.5)
  (`KismetSystemLibrary.Delay` 0.2)
  (`GameplayStatics.SpawnEmitterAtLocation` "/Game/VFX_Toolkit_V1/ParticleSystems/356Days/Par_MatraBoom_01.Par_MatraBoom_01" _returnvalue (`KismetMathLibrary.Conv_VectorToRotator` _returnvalue) (5.0 5.0 5.0))
  (`GameplayStatics.SpawnEmitterAtLocation` "/Game/VFX_Toolkit_V1/ParticleSystems/356Days/Par_Meteora_Explode_01.Par_Meteora_Explode_01" _returnvalue (`KismetMathLibrary.Conv_VectorToRotator` _returnvalue))
  (`PlayerController.ClientStartCameraShake` :`self` (`GameplayStatics.GetPlayerController` 0) :`Shake` "/Game/Blueprint/CameraShakeWeapon.CameraShakeWeapon_C" :`Scale` 0.5)
  (`|SpawnActorFromClass` "/Game/Blueprint/Explosion.Explosion_C" (`KismetMathLibrary.Conv_VectorToTransform` (`SceneComponent.K2_GetComponentLocation` (`self.Barrel`))) "Undefined" "OverrideRootScale" null null)
  (`PlayerController.ClientStartCameraShake` :`self` (`GameplayStatics.GetPlayerController` 0) :`Shake` "/Game/Blueprint/CameraShakeWeapon.CameraShakeWeapon_C" :`Scale` 1.2)
  (`self.K2_DestroyActor`))

(event `self.ReceiveBeginPlay`
  (`ActorComponent.Deactivate` (`self.ParticleSystem`)))

(fn `UserConstructionScript`)