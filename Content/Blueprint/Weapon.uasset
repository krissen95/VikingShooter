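; Weapon Blueprint that fires Laser actors automatically while its trigger is held.
; PullTrigger passes through a DoOnce, fires immediately, then starts a looping timer that calls Fire at an interval derived from RoundsPerSecond.
; Fire spawns a Laser at the ProjectileSpawnPoint transform.
; RealeseTrigger clears the timer and resets the DoOnce, so the next pull fires immediately with no separate cooldown.
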(event `Pull Trigger`
  (`/Engine/EditorBlueprintResources/StandardMacros.DoOnce` false :!label _label
    (:`Completed`
      (`self.Fire`)
      (`KismetSystemLibrary.K2_SetTimer` null "Fire" (/ 1.0 (`self.Rounds Per Second`)) true))))

(event `Realese Trigger`
  (`KismetSystemLibrary.K2_ClearTimer` null "Fire")
  (goto _label :!via `Reset`))

(event `Fire`
  (`|SpawnActorFromClass` "/Game/Blueprint/Laser.Laser_C" (`SceneComponent.K2_GetComponentToWorld` (`self.ProjectileSpawnPoint`)) "Undefined" "OverrideRootScale" null null))

(fn `UserConstructionScript`)