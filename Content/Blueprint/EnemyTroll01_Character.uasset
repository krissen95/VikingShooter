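; Troll enemy character for a twin-stick game that hurts the player on contact and can be killed.
; Overlapping its Collider calls PlayerDamage on the twin-stick character; no knockback is applied here, despite the graph comment.
; AffectHealth runs CalculateHealth, prints Health, then plays an explosion sound and destroys the actor when IsDead.
; The construction script creates a dynamic material instance on the mesh and tints BodyColor red.
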(event `self.collider.OnComponentBeginOverlap`
  (params (OverlappedComponent :type "PrimitiveComponent Object Reference") (OtherActor :type "Actor Object Reference") (OtherComp :type "PrimitiveComponent Object Reference") (OtherBodyIndex :type Integer) (bFromSweep :type Boolean) (SweepResult :type "HitResult Structure (by ref)"))
  ;[1 1 1] Damage and knockback
  (bind _asbp_twin_stick_character (cast `/Game/Blueprint/BP_TwinStickCharacter` OtherActor))
  (`/Game/Blueprint/BP_TwinStickCharacter.PlayerDamage` _asbp_twin_stick_character))

(event `/Game/Blueprint/iDamageable.AffectHealth`
  (params (Delta :type "Float (single-precision)"))
  ;[1 1 1] Take damage and destroy actor
  (`self.CalculateHealth` Delta)
  (`KismetSystemLibrary.PrintString` (`KismetStringLibrary.Conv_DoubleToString` (`self.Health`)))
  (if (`self.isDead`)
    (`GameplayStatics.SpawnSoundAttached` "/Game/VFX_Toolkit_V1/Sounds/S_Explode_Reverb_02.S_Explode_Reverb_02")
    (`self.K2_DestroyActor`)))

(fn `UserConstructionScript`
  (bind _returnvalue (`PrimitiveComponent.CreateDynamicMaterialInstance` (`self.Mesh`) 0 null))
  (bind _output_get (set `self.DynoMat` _returnvalue))
  (`MaterialInstanceDynamic.SetVectorParameterValue` _output_get "BodyColor" (struct :`R` 1.0 :`G` 0.009844 :`A` 1.0)))